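; Game mode that runs the game flow from main menu through play to game over and restart.
; It builds the UI screens, switches camera, input mappings and music, and counts popups to gate player input.
; Temple stages spend data-table resource costs from PlayerData to upgrade abilities, winning at the last stage.
; Tick ends the game when fuel drops below zero; its day-clock call is disconnected.
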(event EventBeginPlay
  (Class|PlayerDataComponent|InitializePlayerData (Variables|Default|GetPlayerData) (Variables|Default|GetDefaultPlayerData))
  (UI|InitializeHudScreen)
  (UI|InitializeMainMenuScreen)
  (UI|InitializeLoadingScreen)
  (UI|InitializeGameOverScreen)
  (bind _returnvalue (Actor|GetActorOfClass "/Script/Engine.CameraActor"))
  (bind _output_get (Variables|Default|SetSceneCamera _returnvalue))
  (UI|StopPlayerInput)
  (Game|Player|SetViewTargetwithBlend (Game|GetPlayerController 0) _output_get 0.0 "VTBlend_Linear" 0.0 false)
  (CallFunction|PlayBGM))

(event EventTick
  (params (DeltaSeconds :type Float%20%28single-precision%29))
  (if (and (< (Class|PlayerDataComponent|GetPlayerAbilityPropertyValue (Variables|Default|GetPlayerData) "EPAPT_CurrentFuel") 0.0) (not (Variables|Default|GetbIsGameOver)))
    (UI|ShowGameoverScreen "EGOT_FuelEmpty")
    (Variables|Default|SetbIsGameOver true)))

(fn ConstructionScript)

(fn IncreaseTime
  (params (Deltatime :type Float%20%28double-precision%29))
  (bind _playerdata (Variables|Default|GetPlayerData))
  (bind _playerdata_2 (Variables|Default|GetPlayerData))
  (bind _output_get (Variables|Time|SetCurrentInterval (+ (* Deltatime (Variables|Time|GetTimeScale)) (Variables|Time|GetCurrentInterval))))
  (if (>= _output_get (Variables|Time|GetTimeInterval))
    (Variables|Time|SetCurrentInterval 0.0)
    (Class|PlayerDataComponent|ChangePlayerCurrentTimeValue _playerdata (+ (Class|PlayerDataComponent|GetPlayerCurrentTimeValue _playerdata) (Variables|Time|GetTimeInterval)))
    (if (>= (Class|PlayerDataComponent|GetPlayerCurrentTimeValue (Variables|Default|GetPlayerData)) (* (Class|KismetSystemLibrary|MakeLiteralInteger 60) 24))
      (Class|PlayerDataComponent|ChangePlayerCurrentTimeValue (Variables|Default|GetPlayerData))
      (if (== (Class|PlayerDataComponent|GetPlayerRemainDaysValue (Variables|Default|GetPlayerData)) 0)
        (CallFunction|RestartGame)
        (elif (< (Class|PlayerDataComponent|GetPlayerRemainDaysValue (Variables|Default|GetPlayerData)) 0)
          (Development|PrintString "PCGGameMode Error: RemainDays is less than 0!" true true "(R=1.000000,G=0.000000,B=0.095176,A=1.000000)")
          (else
            (Class|PlayerDataComponent|ChangePlayerRemainDaysValue _playerdata_2 (- (Class|PlayerDataComponent|GetPlayerRemainDaysValue _playerdata_2) 1))))))))

(fn RestartGame
  (bind _loadingscreen (Variables|UI|GetLoadingScreen))
  (UI|ShowLoadingScreen)
  (Default|StartLoading _loadingscreen)
  (EventDispatchers|BindEventtoOnLoadingComplete _loadingscreen (EventDispatchers|CreateEvent :!event OnLoadingComplete))
  (bind _returnvalue (Actor|GetActorOfClass "/Script/Engine.PlayerStart"))
  (Transformation|SetActorTransform (Game|Player|GetPlayerPawn 0) (Transformation|GetActorTransform _returnvalue) false true)
  (Utilities|Time|SetTimerbyEvent (EventDispatchers|CreateEvent :!event StartLoad) 0.5))

(fn ShowMouseCursor
  (bind _returnvalue (Game|GetPlayerController 0))
  (Variables|/Script/Engine.PlayerController|SetbShowMouseCursor _returnvalue true)
  (Input|SetIgnoreLookInput _returnvalue true))

(fn HideMouseCursor
  (bind _returnvalue (Game|GetPlayerController 0))
  (Variables|/Script/Engine.PlayerController|SetbShowMouseCursor _returnvalue false)
  (Input|SetIgnoreLookInput _returnvalue false))

(fn GetTempleStageRequiredResource
  (params (TempleStage :type Integer))
  (bind _requiredresourcedatatable (Variables|Default|GetRequiredResourceDataTable))
  (bind _outrownames (DataTable|GetDataTableRowNames _requiredresourcedatatable))
  (bind _returnvalue (Utilities|GetDataTableRow _requiredresourcedatatable (Utilities|Array|Get(acopy) _outrownames TempleStage))
    (:then
      (return _returnvalue))
    (:RowNotFound
      (Development|PrintString "GetTempleStageRequiredResourceFailed" true true "(R=1.000000,G=0.000000,B=0.067453,A=1.000000)" 1e+01))))

(fn GetTempleStagePlayerAbilityProperty
  (params (Stage :type Integer))
  (bind _playerabilityupgradeinfo (Variables|UI|GetPlayerAbilityUpgradeInfo))
  (bind _outrownames (DataTable|GetDataTableRowNames _playerabilityupgradeinfo))
  (bind _returnvalue (Utilities|GetDataTableRow _playerabilityupgradeinfo (Utilities|Array|Get(acopy) _outrownames Stage))
    (:then
      (return _returnvalue))))

(fn TrySubmitRequiredResource
  (bind _playerdata (Variables|Default|GetPlayerData))
  (bind _playerdata_2 (Variables|Default|GetPlayerData))
  (bind _requiredresourceinfo (CallFunction|GetTempleStageRequiredResource (Class|PlayerDataComponent|GetPlayerCurrentTempleStageValue (Variables|Default|GetPlayerData))))
  (for _array_element (.requiredresource _requiredresourceinfo)
    (if (< (Class|PlayerDataComponent|GetPlayerResourceValue (Variables|Default|GetPlayerData) (.resourcetype _array_element)) 0)
      (Development|PrintString "TrySubmitRequiredResource: Player Has no such resource type" true true "(R=1.000000,G=0.036018,B=0.000000,A=1.000000)" 1e+01)
      (return false)
      (elif (not (>= (Class|PlayerDataComponent|GetPlayerResourceValue (Variables|Default|GetPlayerData) (.resourcetype _array_element)) (.value _array_element)))
        (Development|PrintString "Required resource not fulfilled ")
        (return false))))
  (for _array_element_2 (.requiredresource _requiredresourceinfo)
    (Class|PlayerDataComponent|ChangePlayerResourceValue _playerdata (.resourcetype _array_element_2) (- (Class|PlayerDataComponent|GetPlayerResourceValue _playerdata (.resourcetype _array_element_2)) (.value _array_element_2)))
    (bind _isgameover (CallFunction|CheckGameWin))
    (if _isgameover
      (UI|ShowGameoverScreen "EGOT_Win")
      (Variables|Default|SetbIsGameOver true)
      (return false)
      (else
        (CallFunction|UpgradePlayerAbility (Class|PlayerDataComponent|GetPlayerCurrentTempleStageValue (Variables|Default|GetPlayerData)))
        (Class|PlayerDataComponent|ChangePlayerCurrentTempleStageValue _playerdata_2 (+ (Class|PlayerDataComponent|GetPlayerCurrentTempleStageValue _playerdata_2) 1))
        (return true)))))

(fn CheckGameWin
  (bind _outrownames (DataTable|GetDataTableRowNames (Variables|Default|GetRequiredResourceDataTable)))
  (return (>= (+ (Class|PlayerDataComponent|GetPlayerCurrentTempleStageValue (Variables|Default|GetPlayerData)) 1) (Utilities|Array|Length _outrownames))))

(fn UpgradePlayerAbility
  (params (TempleStage :type Integer))
  (bind _abilityupgradeitem (CallFunction|GetTempleStagePlayerAbilityProperty TempleStage))
  (for _array_element (.propertyitem _abilityupgradeitem)
    (Class|PlayerDataComponent|ChangePlayerAbilityPropertyValue (Variables|Default|GetPlayerData) (.propertytype _array_element) (+ (.increasevalue _array_element) (Class|PlayerDataComponent|GetPlayerAbilityPropertyValue (Variables|Default|GetPlayerData) (.propertytype _array_element))))))

(fn InitializeHudScreen
  (bind _defaultplayerdata (Variables|Default|GetDefaultPlayerData))
  (bind _returnvalue (Game|ConstructObjectfromClass "/Game/Blueprints/UI/Screen/WBP_HUDScreen.WBP_HUDScreen_C"))
  (bind _output_get (Variables|UI|SetHUDScreen _returnvalue))
  (UserInterface|Viewport|AddtoViewport _returnvalue 0)
  (Default|InitializeHUD _returnvalue (.playerstatus _defaultplayerdata) (.systemstatus _defaultplayerdata) (Variables|Default|GetPlayerData) self)
  (Widget|SetVisibility (Variables|UI|GetHUDScreen) "Hidden"))

(fn GameStartClicked
  (Widget|SetVisibility (Variables|UI|GetMainMenuScreen) "Hidden")
  (Widget|SetVisibility (Variables|UI|GetHUDScreen) "Visible")
  (Game|Player|SetViewTargetwithBlend (Game|GetPlayerController 0) (Game|Player|GetPlayerPawn 0) 1.0 "VTBlend_Linear" 0.0 false)
  (Utilities|Time|SetTimerbyEvent (EventDispatchers|CreateEvent :!event OnStartGameTransitionEnd) 1.0)
  (CallFunction|PlayBGM 1))

(fn ExitGameClicked
  (Game|QuitGame 0 "Quit" false))

(fn InitializeMainMenuScreen
  (bind _returnvalue (Game|ConstructObjectfromClass "/Game/Blueprints/UI/Screen/WBP_MainMenuScreen.WBP_MainMenuScreen_C"))
  (bind _output_get (Variables|UI|SetMainMenuScreen _returnvalue))
  (UserInterface|Viewport|AddtoViewport _output_get 0)
  (Default|InitializeMainMenu (Variables|UI|GetMainMenuScreen) self))

(fn ShowGameoverScreen
  (params (GameOverType :type EGameOverType%20Enum :default "EGOT_Win"))
  (Default|InitializeGameOverScreen (Variables|UI|GetGameOverScreen) self GameOverType)
  (Widget|SetVisibility (Variables|UI|GetHUDScreen) "Hidden")
  (Widget|SetVisibility (Variables|UI|GetGameOverScreen) "Visible")
  (UI|StopPlayerInput)
  (CallFunction|StopBGM))

(fn StopPlayerInput
  (bind _returnvalue (Game|GetPlayerController 0))
  (bind _returnvalue_2 (PlayerController|LocalPlayerSubsystems|GetEnhancedInputLocalPlayerSubsystem _returnvalue))
  (Input|RemoveMappingContext _returnvalue_2 "/Game/ThirdPerson/Input/IMC_Default.IMC_Default" "(bIgnoreAllPressedKeysUntilRelease=True,bForceImmediately=False,bNotifyUserSettings=False)")
  (Input|AddMappingContext _returnvalue_2 "/Game/ThirdPerson/Input/IMC_Menu.IMC_Menu" 0 "(bIgnoreAllPressedKeysUntilRelease=True,bForceImmediately=False,bNotifyUserSettings=False)")
  (Utilities|Time|SetTimerbyEvent (EventDispatchers|CreateEvent :!event UIInputMode) 0.1))

(fn ResumePlayerInput
  (bind _returnvalue (Game|GetPlayerController 0))
  (bind _returnvalue_2 (PlayerController|LocalPlayerSubsystems|GetEnhancedInputLocalPlayerSubsystem _returnvalue))
  (Input|RemoveMappingContext _returnvalue_2 "/Game/ThirdPerson/Input/IMC_Menu.IMC_Menu" "(bIgnoreAllPressedKeysUntilRelease=True,bForceImmediately=False,bNotifyUserSettings=False)")
  (Input|AddMappingContext _returnvalue_2 "/Game/ThirdPerson/Input/IMC_Default.IMC_Default" 0 "(bIgnoreAllPressedKeysUntilRelease=True,bForceImmediately=False,bNotifyUserSettings=False)")
  (Utilities|Time|SetTimerbyEvent (EventDispatchers|CreateEvent :!event PlayInputMode) 0.1))

(fn ShowLoadingScreen
  (Widget|SetVisibility (Variables|UI|GetGameOverScreen) "Hidden")
  (Widget|SetVisibility (Variables|UI|GetLoadingScreen) "Visible"))

(fn InitializeLoadingScreen
  (bind _returnvalue (Game|ConstructObjectfromClass "/Game/Blueprints/UI/Screen/WBP_LoadingScreen.WBP_LoadingScreen_C"))
  (bind _output_get (Variables|UI|SetLoadingScreen _returnvalue))
  (UserInterface|Viewport|AddtoViewport _output_get 10)
  (Widget|SetVisibility (Variables|UI|GetLoadingScreen) "Hidden"))

(fn InitializeGameOverScreen
  (bind _returnvalue (Game|ConstructObjectfromClass "/Game/Blueprints/UI/Screen/WBP_GameoverScreen.WBP_GameoverScreen_C"))
  (bind _output_get (Variables|UI|SetGameOverScreen _returnvalue))
  (UserInterface|Viewport|AddtoViewport _output_get 10)
  (Widget|SetVisibility (Variables|UI|GetGameOverScreen) "Hidden")
  (Default|InitializeGameOverScreen (Variables|UI|GetGameOverScreen) self "EGOT_Win"))

(fn OnLoadingComplete
  (UI|ResumePlayerInput)
  (Widget|SetVisibility (Variables|UI|GetLoadingScreen) "Hidden")
  (Widget|SetVisibility (Variables|UI|GetHUDScreen) "Visible")
  (Variables|Default|SetbIsGameOver false)
  (Variables|Default|SetPopupCounter 0)
  (CallFunction|PlayBGM 1))

(fn GetFTUEManager
  (bind _ftuemanager (Variables|Default|GetFTUEManager)
    (:then
      (return _ftuemanager))
    (:else
      (bind _returnvalue (Actor|GetActorOfClass "/Game/Blueprints/FTUE/BP_FTUEManager.BP_FTUEManager_C"))
      (bind _output_get (Variables|Default|SetFTUEManager _returnvalue))
      (return _output_get))))

(fn StartLoad
  (bind _defaultplayerdata (Variables|Default|GetDefaultPlayerData))
  (Class|PlayerDataComponent|InitializePlayerData (Variables|Default|GetPlayerData) (Variables|Default|GetDefaultPlayerData))
  (Default|InitializeHUD (Variables|UI|GetHUDScreen) (.playerstatus _defaultplayerdata) (.systemstatus _defaultplayerdata) (Variables|Default|GetPlayerData) self)
  (CallFunction|HideMouseCursor)
  (Class|PCGGameMode|HidePopup)
  (EventDispatchers|CallOnTimeZeroGameOver (Variables|Default|GetPlayerData) "/Script/PCG.PlayerDataComponent" "EGOT_Win"))

(fn OnStartGameTransitionEnd
  (Default|ActivateTutorialChain (FTUE|GetFTUEManager) "ETT_InitialTutorial"))

(fn UIInputMode
  (bind _returnvalue (Game|GetPlayerController 0))
  (Variables|/Script/Engine.PlayerController|SetbShowMouseCursor _returnvalue true)
  (Input|SetInputModeUIOnly _returnvalue 0 "DoNotLock" true))

(fn PlayInputMode
  (bind _returnvalue (Game|GetPlayerController 0))
  (Variables|/Script/Engine.PlayerController|SetbShowMouseCursor _returnvalue false)
  (Input|SetInputModeGameOnly _returnvalue true))

(fn AddPopupCounter
  (Math|Integer|IncrementInt (Variables|Default|GetPopupCounter)
    (:%20%20
      (UI|StopPlayerInput))))

(fn SubtractPopupCounter
  (bind _result (Math|Integer|DecrementInt (Variables|Default|GetPopupCounter))
    (:%20%20
      (if (== _result 0)
        (UI|ResumePlayerInput)))))

(fn ShowPauseGame)

(fn PlayBGM
  (params (Input :type Integer))
  (bind _currentbgm (Variables|Default|GetCurrentBGM)
    (:then
      (Audio|Components|Audio|FadeOut _currentbgm 0.5 0.0 "Linear" :!class /Script/Engine.AudioComponent))
    (:else
      _))
  (bind _returnvalue (Audio|CreateSound2D (Utilities|Array|Get(acopy) (Variables|Default|GetBGMs) Input) 1.0 1.0 0.0 0))
  (bind _output_get (Variables|Default|SetCurrentBGM _returnvalue))
  (Audio|Components|Audio|FadeIn _output_get 0.5 1.0 0.0 "Linear" :!class /Script/Engine.AudioComponent))

(fn StopBGM
  (bind _currentbgm (Variables|Default|GetCurrentBGM)
    (:then
      (Audio|Components|Audio|FadeOut _currentbgm 0.5 0.0 "Linear" :!class /Script/Engine.AudioComponent))
    (:else)))