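; Procedural planet actor that builds noisy spherical terrain with Geometry Script and sizes a sea-water sphere to match.
; RefreshPlanet sets a flag and marks the planet for refresh, so GeneratePlanet only rebuilds when flagged.
; Generation derives the radius from RadiusKm, tessellates a box sphere, displaces it along normals with randomly seeded Perlin noise, then updates collision.
; Vertex selection and editing nodes are unconnected leftovers.
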(event Custom|RefreshPlanet
  (Variables|Default|SetRefresh true)
  (Class|GeometryPlanet|MarkPlanetRefresh true true))

(event EventBeginPlay
  (Input|EnableInput (Game|GetPlayerController 0)))

(event Collision|EventActorBeginOverlap
  (params (OtherActor :type Actor%20Object%20Reference)))

(event EventTick
  (params (DeltaSeconds :type Float%20%28single-precision%29)))

(event EventGeneratePlanet
  (params (TargetMesh :type Dynamic%20Mesh%20Object%20Reference))
  (if (Variables|Default|GetRefresh)
    (Variables|Default|SetRefresh false)
    (CallFunction|UpdatePlanet)
    (bind _returnvalue (Class|GeometryScriptLibraryMeshPrimitiveFunctions|AppendSphereBox :TargetMesh TargetMesh :Radius (Variables|Default|GetRadius) :StepsX 30 :StepsY 30 :StepsZ 30 :Debug 0))
    (bind _returnvalue_2 (Class|GeometryScriptLibraryMeshSubdivideFunctions|ApplyUniformTessellation _returnvalue 3 0))
    (bind _outmesh (CallFunction|ApplyPerlinNoise _returnvalue_2 1e+03 0.02 true))
    (Class|GeometryScriptLibraryCollisionFunctions|SetDynamicMeshCollisionfromMesh :FromDynamicMesh _outmesh :ToDynamicMeshComponent (Variables|DynamicMeshActor|GetDynamicMeshComponent) :Debug 0)))

(event Input|MouseEvents|DebugKeyLeftMouseButton
  (params (Key :type Key%20Structure :default "None") (ActionValue :type Input%20Action%20Value%20Structure)))

(fn ConstructionScript)

(fn ApplyPerlinNoise
  (params (TargetMesh :type Dynamic%20Mesh%20Object%20Reference) (Magnitude :type Float%20%28double-precision%29) (Frequency :type Float%20%28double-precision%29) (Randomnize :type Boolean))
  (bind _returnvalue (Class|GeometryScriptLibraryMeshDeformFunctions|ApplyPerlinNoisetoMesh :TargetMesh TargetMesh :Options (Utilities|Struct|MakeGeometryScriptPerlinNoiseOptions (Utilities|Struct|MakeGeometryScriptPerlinNoiseLayerOptions Magnitude Frequency "0.000000,0.000000,0.000000" (Math|Integer|SelectInt (Math|Random|RandomInteger 5000) 0 Randomnize)) true "FullMeshSelection") :Debug 0))
  (return _returnvalue))

(fn UpdatePlanet
  (bind _planetsphere (Variables|Default|GetPlanetSphere))
  (bind (_min _max) (Components|StaticMesh|GetLocalBounds _planetsphere))
  (Variables|Default|SetRadius (* (Variables|Planet|GetRadius%28km%29) 1e+03))
  ;[0.15 0.15 0.15 0.5] 根据星球大小计算海水scale
  (Transformation|SetWorldScale3D (Variables|Default|GetPlanetSphere) (Math|Conversions|ToVector(Float) (* (Variables|Default|GetRadius) (/ 2.0 (- (.x _max) (.x _min)))))))