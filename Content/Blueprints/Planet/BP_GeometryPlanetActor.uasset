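; Procedural planet actor that builds a noise-displaced sphere-box dynamic mesh with collision, wood and fuel foliage, and stone and ore mine spheres.
; RefreshPlanet sets a flag that gates GeneratePlanet, which derives radius from planet data, scales the sea sphere, rebuilds terrain and respawns foliage.
; The time-zero game-over event triggers a refresh and mine respawn.
; Laser hits forward to instanced-mesh components through CollectableItemInterface; older inline foliage logic remains disconnected.
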(event Custom|RefreshPlanet
  (Variables|Default|SetRefresh true)
  (Class|GeometryPlanetActor|MarkPlanetRefresh true true))

(event Custom|SpawnFoliage
  (Default|InitializeISM (Variables|Default|GetBP_WoodISM) self)
  (Default|InitializeISM (Variables|Default|GetBP_FuelISM) self))

(event Custom|CustomEvent
  (params (DataClassType :type Object%20Class%20Reference) (eGameOverType :type EGameOverType%20Enum :default "EGOT_Win"))
  (CallFunction|RefreshPlanet)
  (Class|GeometryPlanetActor|SpawnStoneMineSpheres)
  (Class|GeometryPlanetActor|SpawnOreMineSpheres)
  (Class|GeometryPlanetActor|UpdateMineAreas)
  (EventDispatchers|CallOnPlanetInitialized))

(event EventBeginPlay
  (bind _aspcggame_mode (Utilities|Casting|CastToPCGGameMode (Game|GetGameMode)))
  (EventDispatchers|BindEventtoOnTimeZeroGameOver (Variables|/Script/PCG.PCGGameMode|GetPlayerData _aspcggame_mode) (delegate Custom|CustomEvent))
  (Class|GeometryPlanetActor|InitializePlanet (Variables|Default|GetTestPlanetData))
  (CallFunction|UpdatePlanetRadius)
  (Class|GeometryPlanetActor|SpawnStoneMineSpheres)
  (Class|GeometryPlanetActor|SpawnOreMineSpheres)
  (Class|GeometryPlanetActor|UpdateMineAreas)
  (EventDispatchers|CallOnPlanetInitialized)
  (Utilities|FlowControl|Delay 1.0))

(event Collision|EventActorBeginOverlap
  (params (OtherActor :type Actor%20Object%20Reference)))

(event EventGeneratePlanet
  (params (TargetMesh :type Dynamic%20Mesh%20Object%20Reference))
  (bind _planetresolution (Variables|Default|GetPlanetResolution))
  (if (Variables|Default|GetRefresh)
    (Variables|Default|SetRefresh false)
    (Class|GeometryPlanetActor|InitializePlanet (Variables|Default|GetTestPlanetData))
    (CallFunction|UpdatePlanetRadius)
    (bind _returnvalue (Class|GeometryScriptLibraryMeshPrimitiveFunctions|AppendSphereBox :TargetMesh TargetMesh :Radius (Variables|Default|GetRadius) :StepsX (.x _planetresolution) :StepsY (.y _planetresolution) :StepsZ (.z _planetresolution) :Debug 0))
    (bind _returnvalue_2 (Class|GeometryPlanetActor|ApplyNoisetoPlanet))
    (Class|DynamicMeshComponent|SetDynamicMesh (Variables|DynamicMeshActor|GetDynamicMeshComponent) _returnvalue_2)
    (Class|GeometryScriptLibraryCollisionFunctions|SetDynamicMeshCollisionfromMesh :FromDynamicMesh _returnvalue_2 :Debug 0)
    (bind _returnvalue_3 (DynamicMeshComponent|GetDynamicMesh (Variables|DynamicMeshActor|GetDynamicMeshComponent)))
    (GeometryScript|Normals|RecomputeNormals :TargetMesh _returnvalue_3 :bDeferChangeNotifications true :Debug 0)
    (CallFunction|SpawnFoliage)
    (EventDispatchers|CallOnPlanetInitialized)))

(event EventTick
  (params (DeltaSeconds :type Float%20%28single-precision%29)))

(event EventOnGetHitbyLaser
  (params (ISMComponent :type Instanced%20Static%20Mesh%20Component%20Object%20Reference) (ItemIndex :type Integer) (Damage :type Float%20%28single-precision%29))
  ;[0.15 0.15 0.15 0.5] 当foliage被玩家采集时调用
  (if (Utilities|DoesObjectImplementInterface ISMComponent "/Script/PCG.CollectableItemInterface")
    (Class|CollectableItemInterface|OnGetHit(Message) ISMComponent ItemIndex Damage)))

(fn ConstructionScript)

(fn ApplyPerlinNoise
  (params (TargetMesh :type Dynamic%20Mesh%20Object%20Reference) (Magnitude :type Float%20%28double-precision%29) (Frequency :type Float%20%28double-precision%29) (Seed :type Integer))
  (bind _returnvalue (Class|GeometryScriptLibraryMeshDeformFunctions|ApplyPerlinNoisetoMesh :TargetMesh TargetMesh :Options (Utilities|Struct|MakeGeometryScriptPerlinNoiseOptions (Utilities|Struct|MakeGeometryScriptPerlinNoiseLayerOptions Magnitude Frequency "0.000000,0.000000,0.000000" Seed) true "FullMeshSelection") :Debug 0))
  (return _returnvalue))

(fn UpdatePlanetRadius
  (bind _planetspherestaticmesh (Variables|Default|GetPlanetSphereStaticMesh))
  (bind (_min _max) (Components|StaticMesh|GetLocalBounds _planetspherestaticmesh))
  (Variables|Default|SetRadius (* (Variables|Default|GetPlanetRadius) 1e+03))
  ;[0.15 0.15 0.15 0.5] 根据星球大小计算海水scale
  (Transformation|SetWorldScale3D (Variables|Default|GetPlanetSphereStaticMesh) (Math|Conversions|ToVector(Float) (* (Variables|Default|GetRadius) (/ 2.02 (- (.x _max) (.x _min)))))))

(fn InitializeFoliageComponent
  (params (FoliageType :type Foliage%20Type%20Instanced%20Static%20Mesh%20Object%20Reference)))

(fn GetPlayerData
  (bind _playerdata (Variables|Default|GetPlayerData)
    (:then
      (return _playerdata))
    (:else
      (bind _asbp_pcggame_mode (Utilities|Casting|CastToBP_PCGGameMode (Game|GetGameMode)))
      (bind _output_get (Variables|Default|SetGameMode _asbp_pcggame_mode))
      (bind _output_get_2 (Variables|Default|SetPlayerData (Variables|/Script/PCG.PCGGameMode|GetPlayerData _output_get)))
      (return _output_get_2))))