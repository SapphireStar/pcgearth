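; BP_FuelISM is a collectable fuel resource on planets, apparently an instanced-mesh variant, that refills the player's fuel.
; When collected, it adds fuel in proportion to the X scale of the last destroyed instance, read from LastDestroyedWoodScale.
; It writes the result to the CurrentFuel ability property through player data, capped at FuelMax.
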(event EventBeginPlay
  (|CallParentFunction) ; This node is disabled and will not be called.\nDrag off pins to build functionality.
)

(event EventTick
  (params (DeltaSeconds :type Float%20%28single-precision%29))
  (|CallParentFunction DeltaSeconds) ; This node is disabled and will not be called.\nDrag off pins to build functionality.
)

(event EventOnResourcebeCollected
  (params (ItemIndex :type Integer))
  (bind _newparam (CallFunction|GetPlayerData))
  (bind _lastdestroyedwoodscale (Variables|Default|GetLastDestroyedWoodScale))
  (bind _returnvalue (Class|PlayerDataComponent|GetPlayerAbilityPropertyValue _newparam "EPAPT_CurrentFuel"))
  (bind _returnvalue_2 (Class|PlayerDataComponent|GetPlayerAbilityPropertyValue _newparam "EPAPT_FuelMax"))
  (bind _returnvalue_3 (* 1e+01 (.x _lastdestroyedwoodscale)))
  (bind _returnvalue_4 (+ _returnvalue _returnvalue_3))
  (if (> _returnvalue_4 _returnvalue_2)
    (Class|PlayerDataComponent|ChangePlayerAbilityPropertyValue _newparam "EPAPT_CurrentFuel" _returnvalue_2)
    (else
      (Class|PlayerDataComponent|ChangePlayerAbilityPropertyValue _newparam "EPAPT_CurrentFuel" _returnvalue_4))))