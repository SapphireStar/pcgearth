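; Procedural planet actor that builds a noisy Geometry Script sphere with harvestable foliage.
; On refresh, it scales the sea sphere to the planet radius and displaces a sphere box with two random Perlin passes along normals.
; Foliage spawns as radially aligned instances on mesh vertices, filtered by chance and height band.
; Laser hits drain per-instance health, hide depleted instances by zero scale and award scale-based Wood to player data.
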(event Custom|RefreshPlanet
  (Variables|Default|SetRefresh true)
  (Class|GeometryPlanetActor|MarkPlanetRefresh true true))

(event Custom|SpawnFoliage
  (CallFunction|ClearFoliage)
  (CallFunction|InitializeFoliageComponent (Variables|Default|GetFoliageType))
  (bind _returnvalue (DynamicMeshComponent|GetDynamicMesh (Variables|DynamicMeshActor|GetDynamicMeshComponent)))
  (for _index (range 0 (- (Class|GeometryScriptLibraryMeshQueryFunctions|GetVertexCount _returnvalue) 1))
    (if (.bIsValidVertex (Class|GeometryScriptLibraryMeshQueryFunctions|GetVertexPosition _returnvalue _index))
      (Utilities|CheckifSpawnFoliage (Math|Random|RandomFloat) (.ReturnValue (Class|GeometryScriptLibraryMeshQueryFunctions|GetVertexPosition _returnvalue _index)) (Variables|Default|GetFoliageType)
        (:output
          (Transformation|SetWorldLocationAndRotation (Variables|Default|GetCalcRoot) (+ (.ReturnValue (Class|GeometryScriptLibraryMeshQueryFunctions|GetVertexPosition _returnvalue _index)) (Transformation|GetActorLocation)) (Math|Rotator|MakeRotfromZ (Math|Vector|Normalize (.ReturnValue (Class|GeometryScriptLibraryMeshQueryFunctions|GetVertexPosition _returnvalue _index)))) false true)
          (Transformation|SetRelativeRotation (Variables|Default|GetCalcChild) (Math|Rotator|MakeRotator 0.0 0.0 (Math|Random|RandomFloatinRange 0.0 3.6e+02)) false true)
          (Components|InstancedStaticMesh|AddInstance (Variables|Default|GetISM-Foliage) (Math|Transform|MakeTransform (Transformation|GetWorldLocation (Variables|Default|GetCalcRoot)) (Transformation|GetWorldRotation (Variables|Default|GetCalcChild)) (* (Math|Random|RandomFloatinRange 1.0 1.5) "1.000000,1.000000,1.000000")) true)))))
  (Class|GeometryPlanetActor|InitializeISMFoliage (Variables|Default|GetISM-Foliage)))

(event Custom|ClearFoliage
  (Variables|Default|GetISM-Foliage
    (:then
      (Components|InstancedStaticMesh|ClearInstances (Variables|Default|GetISM-Foliage)))
    (:else)))

(event EventBeginPlay)

(event Collision|EventActorBeginOverlap
  (params (OtherActor :type Actor%20Object%20Reference)))

(event EventGeneratePlanet
  (params (TargetMesh :type Dynamic%20Mesh%20Object%20Reference))
  (if (Variables|Default|GetRefresh)
    (Variables|Default|SetRefresh false)
    (CallFunction|UpdatePlanet)
    (bind _returnvalue (Class|GeometryScriptLibraryMeshPrimitiveFunctions|AppendSphereBox :TargetMesh TargetMesh :Radius (Variables|Default|GetRadius) :StepsX 20 :StepsY 20 :StepsZ 20 :Debug 0))
    (bind _outmesh (CallFunction|ApplyPerlinNoise _returnvalue 1e+03 0.02 true))
    (bind _outmesh_2 (CallFunction|ApplyPerlinNoise _outmesh 5e+01 0.05 true))
    (Class|GeometryScriptLibraryCollisionFunctions|SetDynamicMeshCollisionfromMesh :FromDynamicMesh _outmesh_2 :ToDynamicMeshComponent (Variables|DynamicMeshActor|GetDynamicMeshComponent) :Debug 0)))

(event EventTick
  (params (DeltaSeconds :type Float%20%28single-precision%29)))

(event EventOnGetHitbyLaser
  (params (ISMComponent :type Instanced%20Static%20Mesh%20Component%20Object%20Reference) (ItemIndex :type Integer) (Damage :type Float%20%28single-precision%29))
  (bind _ism_foliage (Variables|Default|GetISM-Foliage))
  (bind _ismfoliageitemshealth (Variables|Default|GetISMFoliageItemsHealth))
  (bind _outinstancetransform (Components|InstancedStaticMesh|GetInstanceTransform _ism_foliage ItemIndex false))
  (bind _output (Utilities|Array|Get(acopy) _ismfoliageitemshealth ItemIndex))
  (bind _returnvalue (- _output Damage))
  ;[0.15 0.15 0.15 0.5] 当foliage被玩家采集时调用
  (if (== ISMComponent (Variables|Default|GetISM-Foliage))
    (Utilities|Array|SetArrayElem (Variables|Default|GetISMFoliageItemsHealth) ItemIndex _returnvalue)
    (if (<= _returnvalue 0.0)
      (Variables|Default|SetLastDestroyedWoodScale (.scale _outinstancetransform))
      (Components|InstancedStaticMesh|UpdateInstanceTransform _ism_foliage ItemIndex (Math|Transform|MakeTransform (.location _outinstancetransform) (.rotation _outinstancetransform) "0.000000,0.000000,0.000000") false false false)
      (bind _playerdata (CallFunction|GetPlayerData))
      (Class|PlayerDataComponent|ChangePlayerResourceValue _playerdata "EFR_Wood" (+ (Class|PlayerDataComponent|GetPlayerResourceValue _playerdata "EFR_Wood") (* (.x (Variables|Default|GetLastDestroyedWoodScale)) 1e+01))))))

(fn ConstructionScript)

(fn ApplyPerlinNoise
  (params (TargetMesh :type Dynamic%20Mesh%20Object%20Reference) (Magnitude :type Float%20%28double-precision%29) (Frequency :type Float%20%28double-precision%29) (Randomnize :type Boolean))
  (bind _returnvalue (Class|GeometryScriptLibraryMeshDeformFunctions|ApplyPerlinNoisetoMesh :TargetMesh TargetMesh :Options (Utilities|Struct|MakeGeometryScriptPerlinNoiseOptions (Utilities|Struct|MakeGeometryScriptPerlinNoiseLayerOptions Magnitude Frequency "0.000000,0.000000,0.000000" (Math|Integer|SelectInt (Math|Random|RandomInteger 5000) 0 Randomnize)) true "FullMeshSelection") :Debug 0))
  (return _returnvalue))

(fn UpdatePlanet
  (bind _planetspherestaticmesh (Variables|Default|GetPlanetSphereStaticMesh))
  (bind (_min _max) (Components|StaticMesh|GetLocalBounds _planetspherestaticmesh))
  (Variables|Default|SetRadius (* (Variables|Default|GetPlanetRadius) 1e+03))
  ;[0.15 0.15 0.15 0.5] 根据星球大小计算海水scale
  (Transformation|SetWorldScale3D (Variables|Default|GetPlanetSphereStaticMesh) (Math|Conversions|ToVector(Float) (* (Variables|Default|GetRadius) (/ 2.02 (- (.x _max) (.x _min)))))))

(fn InitializeFoliageComponent
  (params (FoliageType :type Foliage%20Type%20Instanced%20Static%20Mesh%20Object%20Reference))
  (Variables|Default|GetISM-Foliage
    (:then)
    (:else
      (bind _returnvalue (AddComponent|AddInstancedStaticMeshComponent false))
      (bind _output_get (Variables|Default|SetISM-Foliage _returnvalue))
      (Components|StaticMesh|SetStaticMesh _output_get (Variables|/Script/Foliage.FoliageType_InstancedStaticMesh|GetMesh FoliageType)))))

(fn GetPlayerData
  (bind _playerdata (Variables|Default|GetPlayerData)
    (:then
      (return _playerdata))
    (:else
      (bind _asbp_pcggame_mode (Utilities|Casting|CastToBP_PCGGameMode (Game|GetGameMode)))
      (bind _output_get (Variables|Default|SetGameMode _asbp_pcggame_mode))
      (bind _output_get_2 (Variables|Default|SetPlayerData (Variables|/Script/PCG.PCGGameMode|GetPlayerData _output_get)))
      (return _output_get_2))))