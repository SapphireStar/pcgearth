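; BP_WoodISM is the wood variant of a collectable planet resource, crediting the player with Wood when collected.
; It reports Wood as its resource type through GetCollectableResourceType.
; On collection, it adds to the player's Wood total an amount scaled by the ResourceMultiplier ability and the X scale of the last destroyed wood, so yield follows size.
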(event EventBeginPlay
  (|CallParentFunction))

(event EventTick
  (params (DeltaSeconds :type Float%20%28single-precision%29))
  (|CallParentFunction DeltaSeconds) ; This node is disabled and will not be called.\nDrag off pins to build functionality.
)

(event EventOnResourcebeCollected
  (params (ItemIndex :type Integer))
  (bind _newparam (CallFunction|GetPlayerData))
  (Class|PlayerDataComponent|ChangePlayerResourceValue _newparam "EFR_Wood" (+ (Class|PlayerDataComponent|GetPlayerResourceValue _newparam "EFR_Wood") (* (* (Class|PlayerDataComponent|GetPlayerAbilityPropertyValue _newparam "EPAPT_ResourceMultiplier") (.x (Variables|Default|GetLastDestroyedWoodScale))) 1e+02))))

(fn GetCollectableResourceType
  (return "EFR_Wood"))