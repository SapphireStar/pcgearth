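; Instanced static mesh component that scatters collectable foliage, yielding Wood, over a planet.
; InitializeISM randomly picks planet dynamic mesh vertices within the foliage type's height range, using the planet's helper components to align instances to the radial direction with random yaw.
; Each instance has its own health, reduced by OnGetHit.
; Depleted instances are scaled to zero rather than removed, after saving their scale, then OnResourceBeCollected is called.
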(event EventBeginPlay)

(event EventTick
  (params (DeltaSeconds :type Float%20%28single-precision%29)))

(event EventOnGetHit
  (params (ItemIndex :type Integer) (Damage :type Float%20%28single-precision%29))
  (bind _outinstancetransform (Components|InstancedStaticMesh|GetInstanceTransform ItemIndex false))
  (bind _ismfoliageitemshealth (Variables|Default|GetISMFoliageItemsHealth))
  (bind _output (Utilities|Array|Get(acopy) _ismfoliageitemshealth ItemIndex))
  (bind _returnvalue (- _output Damage))
  (Utilities|Array|SetArrayElem (Variables|Default|GetISMFoliageItemsHealth) ItemIndex _returnvalue)
  (if (<= _returnvalue 0.0)
    (Variables|Default|SetLastDestroyedWoodScale (.scale _outinstancetransform))
    (Components|InstancedStaticMesh|UpdateInstanceTransform ItemIndex (Math|Transform|MakeTransform (.location _outinstancetransform) (.rotation _outinstancetransform) "0.000000,0.000000,0.000000") false false false)
    (Class|CollectableItemInterface|OnResourcebeCollected ItemIndex)))

(fn GetPlayerData
  (bind _playerdata (Variables|Default|GetPlayerData)
    (:then
      (return _playerdata))
    (:else
      (bind _asbp_pcggame_mode (Utilities|Casting|CastToBP_PCGGameMode (Game|GetGameMode)))
      (bind _output_get (Variables|Default|SetPlayerData (Variables|/Script/PCG.PCGGameMode|GetPlayerData _asbp_pcggame_mode)))
      (return _output_get))))

(fn InitializeISM
  (params (Planet :type BP%20Geometry%20Planet%20Actor%20Object%20Reference))
  (bind _foliagetype (Variables|Default|GetFoliageType))
  (bind _height (Variables|/Script/Foliage.FoliageType|GetHeight _foliagetype))
  (Components|StaticMesh|SetStaticMesh (Variables|/Script/Foliage.FoliageType_InstancedStaticMesh|GetMesh (Variables|Default|GetFoliageType)))
  (Variables|Default|SetPlanet Planet)
  (Components|InstancedStaticMesh|ClearInstances)
  (bind _returnvalue (DynamicMeshComponent|GetDynamicMesh (Variables|/Script/PCG.GeometryPlanetActor|GetDynamicMeshComponent Planet)))
  (for _index (range 0 (- (Class|GeometryScriptLibraryMeshQueryFunctions|GetVertexCount _returnvalue) 1))
    (if (.bIsValidVertex (Class|GeometryScriptLibraryMeshQueryFunctions|GetVertexPosition _returnvalue _index))
      (if (and (< (Math|Random|RandomFloat) (Variables|Default|GetFoliageAmount)) (Math|Float|InRange(Float) (- (Math|Vector|VectorLength (.ReturnValue (Class|GeometryScriptLibraryMeshQueryFunctions|GetVertexPosition _returnvalue _index))) (Variables|/Game/Blueprints/Planet/BP_GeometryPlanetActor.BP_GeometryPlanetActor_C|GetRadius Planet)) (.min _height) (.max _height)))
        (Transformation|SetWorldLocationAndRotation (Variables|/Game/Blueprints/Planet/BP_GeometryPlanetActor.BP_GeometryPlanetActor_C|GetCalcRoot Planet) (+ (.ReturnValue (Class|GeometryScriptLibraryMeshQueryFunctions|GetVertexPosition _returnvalue _index)) (Transformation|GetActorLocation Planet)) (Math|Rotator|MakeRotfromZ (Math|Vector|Normalize (.ReturnValue (Class|GeometryScriptLibraryMeshQueryFunctions|GetVertexPosition _returnvalue _index)))) false true)
        (Transformation|SetRelativeRotation (Variables|/Game/Blueprints/Planet/BP_GeometryPlanetActor.BP_GeometryPlanetActor_C|GetCalcChild Planet) (Math|Rotator|MakeRotator 0.0 0.0 (Math|Random|RandomFloatinRange 0.0 3.6e+02)) false true)
        (Components|InstancedStaticMesh|AddInstance (Math|Transform|MakeTransform (Transformation|GetWorldLocation (Variables|/Game/Blueprints/Planet/BP_GeometryPlanetActor.BP_GeometryPlanetActor_C|GetCalcRoot Planet)) (Transformation|GetWorldRotation (Variables|/Game/Blueprints/Planet/BP_GeometryPlanetActor.BP_GeometryPlanetActor_C|GetCalcChild Planet)) (* (Math|Random|RandomFloatinRange 1.0 1.5) "1.000000,1.000000,1.000000")) true))))
  (Development|PrintString (Utilities|String|ToString(Text) (Utilities|Text|FormatText "Spawned {value} foliage" (Components|InstancedStaticMesh|GetInstanceCount))))
  ;[0.15 0.15 0.15 0.5] 初始化所有Instance血量
  (Utilities|Array|Clear (Variables|Default|GetISMFoliageItemsHealth))
  (for _index_2 (range 0 (- (Components|InstancedStaticMesh|GetInstanceCount) 1))
    (Utilities|Array|Add (Variables|Default|GetISMFoliageItemsHealth) 1e+02)))

(fn GetHit)

(fn GetCollectableResourceType
  (return "EFR_Wood"))