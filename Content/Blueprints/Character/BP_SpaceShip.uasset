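; BP_SpaceShip is the player's ship, flying around geometry planets with fuel drain scaled to velocity.
; It acquires a nearby planet and releases it beyond escape range, easing its absolute-rotation mesh upright to the surface normal, or to the spring arm in space.
; Per-tick traces report aimed collectable resources and drive factory and build-grid tooltips.
; With the GetResource ability, input spawns a laser beam whose endpoint follows the camera trace.
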(event Input|EnhancedActionEvents|EnhancedInputActionIA_UseAbility
  (params (ActionValue :type Boolean) (ElapsedSeconds :type Float%20%28double-precision%29) (TriggeredSeconds :type Float%20%28double-precision%29) (InputAction :type Input%20Action%20Object%20Reference :default "/Game/ThirdPerson/Input/Actions/IA_UseAbility.IA_UseAbility"))
  (:Started
    (if (Utilities|Enum|Equal(Enum) (Variables|/Script/PCG.ItemAbilityComponent|GetAbilityType (Variables|Default|GetCurrentAbilityComponent)) "GetResource")
      (bind _returnvalue (Game|SpawnActorfromClass "/Game/BeamAndLaserFX01/Blueprints/BP_ky_beam06.BP_ky_beam06_C" (Math|Transform|MakeTransform (Transformation|GetWorldLocation (Variables|Default|GetFront)) "0, 0, 0" "1.000000,1.000000,1.000000") "AlwaysSpawn" "MultiplyWithRoot" 0 0))
      (bind _output_get (Variables|Default|SetLaserActor _returnvalue))
      (Variables|/Game/BeamAndLaserFX01/Blueprints/BP_ky_beam01.BP_ky_beam01_C|SetisNotLoop _output_get false)
      (Transformation|SetAbsolute (Variables|/Game/BeamAndLaserFX01/Blueprints/BP_ky_beam01.BP_ky_beam01_C|GetDefaultSceneRoot _output_get) false true false)
      (Transformation|AttachActorToActor _output_get self "None" "KeepWorld" "KeepWorld" "KeepWorld" true)
      (Variables|Default|SetLaserEndActor (Variables|/Game/BeamAndLaserFX01/Blueprints/BP_ky_beam01.BP_ky_beam01_C|GetbeamEndTarget _returnvalue)))))

(event Input|EnhancedActionEvents|EnhancedInputActionIA_UseAbility
  (params (ActionValue :type Boolean) (ElapsedSeconds :type Float%20%28double-precision%29) (TriggeredSeconds :type Float%20%28double-precision%29) (InputAction :type Input%20Action%20Object%20Reference :default "/Game/ThirdPerson/Input/Actions/IA_UseAbility.IA_UseAbility"))
  (bind _returnvalue (Transformation|GetActorLocation))
  (bind _laserrange (Variables|Default|GetLaserRange))
  (bind _camera (Variables|Default|GetCamera))
  (bind _returnvalue_2 (Transformation|GetWorldLocation _camera))
  (bind _returnvalue_3 (Math|Vector|GetForwardVector _camera))
  (bind _returnvalue_4 (* _returnvalue_3 _laserrange))
  (bind _returnvalue_5 (+ _returnvalue_2 _returnvalue_4))
  (Variables|Default|GetLaserEndActor
    (:then
      (bind _outhit (Collision|LineTraceByChannel _returnvalue_2 _returnvalue_5 "TraceTypeQuery1" false 0 "None"))
      (if (.bblockinghit _outhit)
        (Transformation|SetActorLocation (Variables|Default|GetLaserEndActor) (.impactpoint _outhit) false false)
        (Transformation|SetActorLocation (Variables|Default|GetLaserActor) _returnvalue false false)
        (else
          (Transformation|SetActorLocation (Variables|Default|GetLaserEndActor) _returnvalue_5 false false)
          (Transformation|SetActorLocation (Variables|Default|GetLaserActor) _returnvalue false false))))
    (:else)))

(event Input|EnhancedActionEvents|EnhancedInputActionIA_UseAbility
  (params (ActionValue :type Boolean) (ElapsedSeconds :type Float%20%28double-precision%29) (TriggeredSeconds :type Float%20%28double-precision%29) (InputAction :type Input%20Action%20Object%20Reference :default "/Game/ThirdPerson/Input/Actions/IA_UseAbility.IA_UseAbility"))
  (:Completed
    (bind _laserendactor (Variables|Default|GetLaserEndActor)
      (:then
        (Transformation|AttachActorToActor _laserendactor self "None" "KeepWorld" "KeepWorld" "KeepWorld" true)
        (Variables|Default|SetLaserEndActor 0)
        (bind _laseractor (Variables|Default|GetLaserActor)
          (:then
            (Transformation|AttachActorToActor _laseractor self "None" "KeepWorld" "KeepWorld" "KeepWorld" true)
            (Variables|/Game/BeamAndLaserFX01/Blueprints/BP_ky_beam01.BP_ky_beam01_C|SetisNotLoop _laseractor true)
            (Variables|Default|SetLaserActor 0))
          (:else)))
      (:else))))

(event EventBeginPlay
  (bind _outactors (Collision|SphereOverlapActors (Transformation|GetActorLocation) 1e+04 (Utilities|Array|MakeArray "ObjectTypeQuery1" "ObjectTypeQuery2") "/Game/Blueprints/Planet/BP_GeometryPlanetActor.BP_GeometryPlanetActor_C"))
  (bind _array_element (Utilities|Array|ForEachLoopwithBreak _outactors :!label _label)
    (:LoopBody
      (bind _asbp_geometry_planet_actor (Utilities|Casting|CastToBP_GeometryPlanetActor _array_element))
      (Variables|Default|SetPlanet _asbp_geometry_planet_actor)
      (goto _label Break))
    (:Completed
      ;[0.15 0.15 0.15 0.5] InitializeTooltip
      (bind _returnvalue (Game|ConstructObjectfromClass "/Game/Blueprints/UI/Tooltip/WBP_ToolTip.WBP_ToolTip_C"))
      (bind _output_get (Variables|Tooltip|SetTooltip _returnvalue))
      (UserInterface|Viewport|AddtoViewport _output_get -1)
      (Widget|SetVisibility _output_get "Hidden")
      (Transformation|SetAbsolute (Variables|Default|GetStaticMesh) false true false)
      (CallFunction|SetMeshInitialiRotation))))

(event Collision|EventActorBeginOverlap
  (params (OtherActor :type Actor%20Object%20Reference)))

(event EventTick
  (params (DeltaSeconds :type Float%20%28single-precision%29))
  (CallFunction|CheckCollectableResourceType)
  (CallFunction|ConsumeFuel)
  (CallFunction|OrbitMove)
  (CallFunction|MeshLerptoRotation)
  (Tooltip|CheckFactory DeltaSeconds)
  (Tooltip|CheckBuildAbilityInfo)
  (CallFunction|CheckOrbit))

(fn ConstructionScript)

(fn CheckCollectableResourceType
  (bind _camera (Variables|Default|GetCamera))
  (bind _returnvalue (Transformation|GetWorldLocation _camera))
  (bind (_outhits _returnvalue_2) (Collision|MultiSphereTraceByChannel _returnvalue (+ _returnvalue (* (Math|Vector|GetForwardVector _camera) (Variables|Default|GetSelectRange))) 0.0 "TraceTypeQuery1" false 0 "None"))
  (if _returnvalue_2
    (bind _array_element (Utilities|Array|ForEachLoopwithBreak _outhits)
      (:LoopBody
        (if (Utilities|DoesObjectImplementInterface (.hitactor _array_element) "/Script/PCG.CollectableItemInterface")
          (bind _returnvalue_3 (Class|CollectableItemInterface|GetCollectableResourceType(Message) (.hitactor _array_element)))
          (EventDispatchers|CallOnPlayerAimingResourceChanged _returnvalue_3)
          (return)
          (elif (Utilities|DoesObjectImplementInterface (.hitcomponent _array_element) "/Script/PCG.CollectableItemInterface")
            (bind _returnvalue_4 (Class|CollectableItemInterface|GetCollectableResourceType(Message) (.hitcomponent _array_element)))
            (EventDispatchers|CallOnPlayerAimingResourceChanged _returnvalue_4)
            (return))))
      (:Completed
        (EventDispatchers|CallOnPlayerAimingResourceChanged "EFR_None")))
    (else
      (EventDispatchers|CallOnPlayerAimingResourceChanged "EFR_None"))))

(fn ConsumeFuel
  (bind _playerdata (Variables|Default|GetPlayerData))
  (bind _playerdata_2 (Variables|Default|GetPlayerData)
    (:then
      (if (>= (Class|PlayerDataComponent|GetPlayerAbilityPropertyValue _playerdata_2 "EPAPT_CurrentFuel") 0.0)
        (Class|PlayerDataComponent|ChangePlayerAbilityPropertyValue _playerdata "EPAPT_CurrentFuel" (- (Class|PlayerDataComponent|GetPlayerAbilityPropertyValue _playerdata "EPAPT_CurrentFuel") (/ (Math|Vector|VectorLength (Transformation|GetComponentVelocity (Variables|Default|GetMainBody))) (* (Variables|Default|GetBaseSpeed) 5e+01))))))
    (:else)))

(fn OrbitMove
  (bind _springarm (Variables|Default|GetSpringArm))
  (Variables|Default|GetPlanet
    (:then
      (bind _output_get (LocalVariables|SetNormal (Math|Vector|Normalize (- (Transformation|GetActorLocation) (Transformation|GetActorLocation (Variables|Default|GetPlanet))))))
      (Variables|Default|SetMeshTargetRotation (Math|Rotator|MakeRotfromZX _output_get (* (Math|Vector|GetRightVector (Variables|Default|GetSpringArm)) -1.0))))
    (:else
      (Variables|Default|SetMeshTargetRotation (Math|Rotator|MakeRotfromZX (Math|Vector|GetUpVector _springarm) (* (Math|Vector|GetRightVector _springarm) -1.0))))))

(fn ShowTooltip
  (params (Input :type Tooltip%20Info%20Structure))
  (bind _tooltip (Variables|Tooltip|GetTooltip)
    (:then
      (Default|ShowTooltip _tooltip Input))
    (:else)))

(fn HideTooltip
  (bind _tooltip (Variables|Tooltip|GetTooltip)
    (:then
      (Widget|SetVisibility _tooltip "Hidden"))
    (:else)))

(fn CheckBuildAbilityInfo
  (if (Class|TerrainBuildAbility|GetIsSelectingGrid (Variables|Default|GetTerrainBuildAbility))
    (bind _returnvalue (Class|TooltipableInterface|GetFactoryTooltipInfo (Variables|Default|GetTerrainBuildAbility)))
    (Tooltip|ShowTooltip _returnvalue)
    (elif (Class|TerrainBuildAbility|GetIsSelectingGrid (Variables|Default|GetTerrainBuildCraftAbility))
      (bind _returnvalue_2 (Class|TooltipableInterface|GetFactoryTooltipInfo (Variables|Default|GetTerrainBuildCraftAbility)))
      (Tooltip|ShowTooltip _returnvalue_2))))

(fn CheckFactory
  (params (Deltatime :type Float%20%28double-precision%29))
  (bind _front (Variables|Default|GetFront))
  (bind _returnvalue (Transformation|GetWorldLocation _front))
  (bind _outhit (Collision|LineTraceByChannel _returnvalue (+ _returnvalue (* (Math|Vector|GetForwardVector (Variables|Default|GetCamera)) (Variables|Default|GetSelectRange))) "TraceTypeQuery5" false 0 "None"))
  (if (.bblockinghit _outhit)
    (if (== (Variables|Tooltip|GetCurFactoryTarget) (.hitactor _outhit))
      (if (> (Variables|Tooltip|GetTooltipCounter) (Variables|Tooltip|GetTooltipCD))
        (Variables|Tooltip|SetTooltipCounter 0.0)
        (bind _returnvalue_2 (Class|TooltipableInterface|GetFactoryTooltipInfo(Message) (Variables|Tooltip|GetCurFactoryTarget)))
        (Tooltip|ShowTooltip _returnvalue_2)
        (else
          (Variables|Tooltip|SetTooltipCounter (+ (Variables|Tooltip|GetTooltipCounter) Deltatime))))
      (else
        (bind _output_get (Variables|Tooltip|SetCurFactoryTarget (.hitactor _outhit)))
        (if (Utilities|DoesObjectImplementInterface (.hitactor _outhit) "/Script/PCG.TooltipableInterface")
          (bind _returnvalue_3 (Class|TooltipableInterface|GetFactoryTooltipInfo(Message) _output_get))
          (Tooltip|ShowTooltip _returnvalue_3))))
    (else
      (Tooltip|HideTooltip)
      (Variables|Tooltip|SetCurFactoryTarget 0))))

(fn CheckTwoTooltipEqual)

(fn CheckOrbit
  (bind _planet (Variables|Default|GetPlanet)
    (:then
      (if (> (Math|Vector|Distance(Vector) (Transformation|GetActorLocation) (Transformation|GetActorLocation _planet)) (+ (Variables|/Game/Blueprints/Planet/BP_GeometryPlanetActor.BP_GeometryPlanetActor_C|GetRadius _planet) (Variables|Default|GetEscapeDist)))
        (Variables|Default|SetPlanet 0)))
    (:else
      (bind _outactors (Collision|SphereOverlapActors (Transformation|GetActorLocation) 4e+03 (Utilities|Array|MakeArray "ObjectTypeQuery1" "ObjectTypeQuery2") "/Game/Blueprints/Planet/BP_GeometryPlanetActor.BP_GeometryPlanetActor_C"))
      (bind _array_element (Utilities|Array|ForEachLoopwithBreak _outactors :!label _label)
        (:LoopBody
          (bind _asbp_geometry_planet_actor (Utilities|Casting|CastToBP_GeometryPlanetActor _array_element))
          (Variables|Default|SetPlanet _asbp_geometry_planet_actor)
          (goto _label Break))))))

(fn MeshLerptoRotation
  (Transformation|SetWorldRotation (Variables|Default|GetStaticMesh) (Math|Rotator|Lerp(Rotator) (Transformation|GetWorldRotation (Variables|Default|GetStaticMesh)) (Variables|Default|GetMeshTargetRotation) 0.2 true) false false))

(fn SetMeshInitialiRotation
  (bind _springarm (Variables|Default|GetSpringArm))
  (Variables|Default|GetPlanet
    (:then
      (bind _output_get (LocalVariables|SetNormal (Math|Vector|Normalize (- (Transformation|GetActorLocation) (Transformation|GetActorLocation (Variables|Default|GetPlanet))))))
      (Transformation|SetWorldRotation (Variables|Default|GetStaticMesh) (Math|Rotator|MakeRotfromZX _output_get (* (Math|Vector|GetRightVector (Variables|Default|GetSpringArm)) -1.0)) false false))
    (:else
      (Variables|Default|SetMeshTargetRotation (Math|Rotator|MakeRotfromZX (Math|Vector|GetUpVector _springarm) (* (Math|Vector|GetRightVector _springarm) -1.0))))))