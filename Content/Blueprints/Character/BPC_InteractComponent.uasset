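; BPC_InteractComponent is a character component meant to detect interactable actors ahead, though its detection logic is currently disconnected and Tick does nothing.
; BeginPlay caches PCGGameMode, and InitializeComponent stores the Front and Camera references.
; The unwired logic sphere-traces along camera forward for BPI_Interactable actors and asks the game mode to show or hide the interact widget.
; Its own ShowInteractWidget and HideInteractWidget functions are empty.
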(event EventBeginPlay
  (bind _aspcggame_mode (Utilities|Casting|CastToPCGGameMode (Game|GetGameMode)))
  (Variables|Default|SetGameMode _aspcggame_mode))

(event EventTick
  (params (DeltaSeconds :type Float%20%28single-precision%29)))

(fn InitializeComponent
  (params (Front :type Primitive%20Component%20Object%20Reference) (Camera :type Camera%20Component%20Object%20Reference))
  (Variables|Default|SetFront Front)
  (Variables|Default|SetCamera Camera)
  (Variables|Default|SetbIsInitialized true))

(fn ShowInteractWidget)

(fn HideInteractWidget)