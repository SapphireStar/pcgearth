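; BP_GridSelection previews a grid selection at the point the player pawn is facing.
; It enables input for player 0 on BeginPlay and runs UpdateGridSelection every Tick.
; That function line-traces forward from the pawn on a dedicated trace channel, ignoring the pawn and drawing a one-frame debug line.
; On a blocking hit, it passes the impact point to PreviewSelectGrid, which is defined outside these graphs.
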(event EventBeginPlay
  (Input|EnableInput (Game|GetPlayerController 0)))

(event Collision|EventActorBeginOverlap
  (params (OtherActor :type Actor%20Object%20Reference)))

(event EventTick
  (params (DeltaSeconds :type Float%20%28single-precision%29))
  (CallFunction|UpdateGridSelection))

(fn ConstructionScript)

(fn UpdateGridSelection
  (bind _returnvalue (Game|Player|GetPlayerPawn 0))
  (bind _returnvalue_2 (Game|Player|GetPlayerPawn 0))
  (bind _returnvalue_3 (Transformation|GetActorLocation _returnvalue))
  (Utilities|IsValid _returnvalue_2
    (:Is%20Valid
      (bind _outhit (Collision|LineTraceByChannel _returnvalue_3 (+ _returnvalue_3 (* (Transformation|GetActorForwardVector _returnvalue) 1e+04)) "TraceTypeQuery3" false (Utilities|Array|MakeArray _returnvalue_2) "ForOneFrame" false))
      (if (.bblockinghit _outhit)
        (Class|GridSelectionManager|PreviewSelectGrid (.impactpoint _outhit))))))