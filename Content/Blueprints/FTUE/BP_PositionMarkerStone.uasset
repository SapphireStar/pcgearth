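; FTUE position marker that relocates itself onto a MineSphereStone in the world.
; GetTarget runs a large-radius sphere overlap around the marker for MineSphereStone actors among static and dynamic world objects.
; It moves the marker to each result in turn, so it ends on the last one returned rather than the nearest.
; The event graph holds no logic of its own, and Tick only calls the parent.
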(event EventBeginPlay
  (|CallParentFunction) ; This node is disabled and will not be called.\nDrag off pins to build functionality.
)

(event Collision|EventActorBeginOverlap
  (params (OtherActor :type Actor%20Object%20Reference))
  (|CallParentFunction OtherActor) ; This node is disabled and will not be called.\nDrag off pins to build functionality.
)

(event EventTick
  (params (DeltaSeconds :type Float%20%28single-precision%29))
  (|CallParentFunction DeltaSeconds))

(fn ConstructionScript
  (|CallParentFunction))

(fn GetTarget
  (bind _outactors (Collision|SphereOverlapActors (Transformation|GetActorLocation) 3e+04 (Utilities|Array|MakeArray "ObjectTypeQuery1" "ObjectTypeQuery2") "/Script/PCG.MineSphereStone"))
  (bind _array_element (Utilities|Array|ForEachLoopwithBreak _outactors)
    (:LoopBody
      (Transformation|SetActorLocation (Transformation|GetActorLocation _array_element) false false))))