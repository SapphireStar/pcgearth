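; FTUE popup tutorial actor for mining ore, built on a parent tutorial class.
; TriggerTutorial creates WBP_MineOrePopup, adds it to the viewport and initializes it with itself, then calls the parent trigger only if the game mode is BP_PCGGameMode.
; OnComplete defers to the parent, followed by a game mode cast that drives nothing.
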(event EventBeginPlay
  (|CallParentFunction) ; This node is disabled and will not be called.\nDrag off pins to build functionality.
)

(event Collision|EventActorBeginOverlap
  (params (OtherActor :type Actor%20Object%20Reference))
  (|CallParentFunction OtherActor) ; This node is disabled and will not be called.\nDrag off pins to build functionality.
)

(event EventTick
  (params (DeltaSeconds :type Float%20%28single-precision%29))
  (|CallParentFunction DeltaSeconds) ; This node is disabled and will not be called.\nDrag off pins to build functionality.
)

(fn ConstructionScript
  (|CallParentFunction))

(fn TriggerTutorial
  (bind _returnvalue (Game|ConstructObjectfromClass "/Game/Blueprints/UI/TutorialPopup/WBP_MineOrePopup.WBP_MineOrePopup_C"))
  (UserInterface|Viewport|AddtoViewport _returnvalue 0)
  (Default|InitializeTutorialPopup _returnvalue self)
  (Utilities|Casting|CastToBP_PCGGameMode (Game|GetGameMode))
  (|CallParentFunction))

(fn OnComplete
  (|CallParentFunction)
  (Utilities|Casting|CastToBP_PCGGameMode (Game|GetGameMode)))