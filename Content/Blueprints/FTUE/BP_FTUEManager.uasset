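; First-time user experience manager that launches tutorial chains as the player reaches wood and temple-stage milestones (submit, mine, craft).
; It binds to PlayerData change events, with check functions choosing which tutorial to activate.
; Activation spawns the chain's actors from FTUEData, links them through NextTutorial and triggers the first.
; Triggered and completed maps block re-triggering an unfinished chain; ClearAllFTUE resets the triggered map.
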(event Custom|TestTutorialChain)

(event EventBeginPlay
  (EventDispatchers|BindEventtoOnPlayerResourceChanged (Variables|/Script/PCG.PCGGameMode|GetPlayerData (CallFunction|GameMode)) (EventDispatchers|CreateEvent :!event CheckFisrtSubmit))
  (EventDispatchers|BindEventtoOnCurrentTempleStageChanged (Variables|/Script/PCG.PCGGameMode|GetPlayerData (CallFunction|GameMode)) (EventDispatchers|CreateEvent :!event CheckFirstMine))
  (EventDispatchers|BindEventtoOnCurrentTempleStageChanged (Variables|/Script/PCG.PCGGameMode|GetPlayerData (CallFunction|GameMode)) (EventDispatchers|CreateEvent :!event CheckFirstCraft)))

(event Collision|EventActorBeginOverlap
  (params (OtherActor :type Actor%20Object%20Reference)))

(event EventTick
  (params (DeltaSeconds :type Float%20%28single-precision%29)))

(fn ConstructionScript)

(fn InitializeFTUEManager
  (bind _asbp_pcggame_mode (Utilities|Casting|CastToBP_PCGGameMode (Game|GetGameMode)))
  (EventDispatchers|BindEventtoOnTimeZeroGameOver (Variables|/Script/PCG.PCGGameMode|GetPlayerData _asbp_pcggame_mode) (EventDispatchers|CreateEvent :!event ClearAllFTUE)))

(fn ClearAllFTUE
  (params (DataClassType :type Object%20Class%20Reference) (eGameOverType :type EGameOverType%20Enum :default "EGOT_Win"))
  (Utilities|Map|Clear (Variables|Default|GetTriggeredFTUEMap)))

(fn ActivateTutorialChain
  (params (TutorialType :type ETutorialType%20Enum :default "ETT_InitialTutorial"))
  (if (not (and (.Value (Utilities|Map|Find (Variables|Default|GetTriggeredFTUEMap) TutorialType)) (not (.Value (Utilities|Map|Find (Variables|Default|GetCompletedFTUEMap) TutorialType)))))
    (Utilities|Map|Add (Variables|Default|GetTriggeredFTUEMap) TutorialType true)
    (bind _returnvalue (Class|FTUEData|GetTutorialChain (Variables|Default|GetFTUEData) TutorialType))
    (for (_array_element _array_index) (.tutorialactorclass _returnvalue)
      (bind _asactor (Utilities|Casting|CastToActorClass _array_element))
      (bind _returnvalue_2 (Game|SpawnActorfromClass _asactor (Transformation|GetActorTransform) "AlwaysSpawn" "MultiplyWithRoot" 0 0))
      (bind _asbp_tutorial_actor_base (Utilities|Casting|CastToBP_TutorialActorBase _returnvalue_2))
      (bind _prevtutorialactor (LocalVariables|GetPrevTutorialActor)
        (:then
          (Variables|/Game/Blueprints/FTUE/BP_TutorialActorBase.BP_TutorialActorBase_C|SetNextTutorial _prevtutorialactor _asbp_tutorial_actor_base))
        (:else
          _))
      (LocalVariables|SetPrevTutorialActor _asbp_tutorial_actor_base)
      ;[0.15 0.15 0.15 0.5] 如果是教程链的第一个元素,那么进行记录,方便之后触发
      (if (== _array_index 0)
        (LocalVariables|SetFirstTutorial _asbp_tutorial_actor_base)))
    (bind _firsttutorial (LocalVariables|GetFirstTutorial)
      (:then
        (Default|TriggerTutorial _firsttutorial))
      (:else))))

(fn DeactivateTutorialChain)

(fn GameMode
  (bind _gamemod (Variables|Default|Getgamemod)
    (:then
      (return _gamemod))
    (:else
      (bind _asbp_pcggame_mode (Utilities|Casting|CastToBP_PCGGameMode (Game|GetGameMode)))
      (bind _output_get (Variables|Default|Setgamemod _asbp_pcggame_mode))
      (return _output_get))))

(fn CheckFisrtSubmit
  (params (ResourceType :type EFactoryResource%20Enum :default "EFR_Wood") (OldValue :type Integer) (NewValue :type Integer))
  (if (and (Utilities|Enum|Equal(Enum) ResourceType "EFR_Wood") (>= NewValue 1000))
    (CallFunction|ActivateTutorialChain "ETT_FirstSubmitTutorial")))

(fn CheckFirstMine
  (params (OldValue :type Integer) (NewValue :type Integer))
  (if (== NewValue 1)
    (CallFunction|ActivateTutorialChain "ETT_MineTutorial")))

(fn CheckFirstCraft
  (params (OldValue :type Integer) (NewValue :type Integer))
  (if (== NewValue 3)
    (CallFunction|ActivateTutorialChain "ETT_CraftTutorial")))