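; Tutorial position marker for the first-time user experience that places itself on a wood resource near the player.
; GetTarget runs a zero-length, large-radius multi-sphere trace on the Visibility channel at the player pawn.
; It takes the first hit on a BP_WoodISM, using the hit item as instance index to move the actor to that instance's world location.
; The event graph is inactive, so GetTarget is not called within this Blueprint.
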(event EventBeginPlay
  (|CallParentFunction) ; This node is disabled and will not be called.\nDrag off pins to build functionality.
)

(event Collision|EventActorBeginOverlap
  (params (OtherActor :type Actor%20Object%20Reference))
  (|CallParentFunction OtherActor) ; This node is disabled and will not be called.\nDrag off pins to build functionality.
)

(event EventTick
  (params (DeltaSeconds :type Float%20%28single-precision%29))
  (|CallParentFunction DeltaSeconds) ; This node is disabled and will not be called.\nDrag off pins to build functionality.
)

(fn ConstructionScript
  (|CallParentFunction))

(fn GetTarget
  (bind _returnvalue (Game|Player|GetPlayerPawn 0))
  (bind _returnvalue_2 (Transformation|GetActorLocation _returnvalue))
  (bind _outhits (Collision|MultiSphereTraceByChannel _returnvalue_2 _returnvalue_2 1e+04 "TraceTypeQuery1" false 0 "None"))
  (bind _array_element (Utilities|Array|ForEachLoopwithBreak _outhits)
    (:LoopBody
      (if (Class|GameplayStatics|ObjectIsA (.hitcomponent _array_element) "/Game/Blueprints/Planet/BP_WoodISM.BP_WoodISM_C")
        (bind _asbp_wood_ism (Utilities|Casting|CastToBP_WoodISM (.hitcomponent _array_element)))
        (Transformation|SetActorLocation (.location (.OutInstanceTransform (Components|InstancedStaticMesh|GetInstanceTransform _asbp_wood_ism (.hititem _array_element) true))) false false)
        (return)))))