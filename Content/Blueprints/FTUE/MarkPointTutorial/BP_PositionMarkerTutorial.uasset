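; Tutorial step actor that puts an on-screen position marker on a mine sphere stone and completes when the player gets close.
; On trigger, it sphere-overlaps for stones, teleports to each so it ends on the last found, then shows a WBP_MarkPoint widget there.
; Once started, Tick compares player distance to TriggerDistance, then removes the marker and destroys the actor.
; GetClosestActor is defined but not called here.
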(event EventBeginPlay
  (|CallParentFunction))

(event Collision|EventActorBeginOverlap
  (params (OtherActor :type Actor%20Object%20Reference))
  (|CallParentFunction OtherActor) ; This node is disabled and will not be called.\nDrag off pins to build functionality.
)

(event EventTick
  (params (DeltaSeconds :type Float%20%28single-precision%29))
  (|CallParentFunction DeltaSeconds)
  (if (Variables|Default|GetbIsTutorialStarted)
    (if (< (Math|Vector|Distance(Vector) (Transformation|GetActorLocation (Game|Player|GetPlayerPawn 0)) (Transformation|GetActorLocation)) (Variables|Default|GetTriggerDistance))
      (CallFunction|OnComplete))))

(fn ConstructionScript
  (|CallParentFunction))

(fn TriggerTutorial
  (|CallParentFunction)
  (CallFunction|GetTarget)
  (bind _returnvalue (Game|ConstructObjectfromClass "/Game/Blueprints/UI/WBP_MarkPoint.WBP_MarkPoint_C"))
  (bind _output_get (Variables|Default|SetMarkPoint _returnvalue))
  (UserInterface|Viewport|AddtoViewport _output_get 0)
  (Default|InitializeMarkPoint (Variables|Default|GetMarkPoint) "/Game/Textures/ScifiUI/Sci-fi_Icon_Pack___Free_iconset__Community___3_/alert-one.alert-one" (Transformation|GetActorLocation)))

(fn OnComplete
  (|CallParentFunction)
  (Widget|RemovefromParent (Variables|Default|GetMarkPoint))
  (Actor|DestroyActor))

(fn GetTarget
  (bind _outactors (Collision|SphereOverlapActors (Transformation|GetActorLocation) 3e+04 (Utilities|Array|MakeArray "ObjectTypeQuery1" "ObjectTypeQuery2") "/Script/PCG.MineSphereStone"))
  (bind _array_element (Utilities|Array|ForEachLoopwithBreak _outactors)
    (:LoopBody
      (Transformation|SetActorLocation (Transformation|GetActorLocation _array_element) false false))))

(fn GetClosestActor
  (params (Actors :type Array%20of%20Actor%20Object%20References))
  (LocalVariables|SetPlayerLocation (Transformation|GetActorLocation (Game|Player|GetPlayerPawn 0)))
  (LocalVariables|SetClosetDist 1e+06)
  (for _array_element Actors
    (if (< (Math|Vector|Distance(Vector) (Transformation|GetActorLocation _array_element) (LocalVariables|GetPlayerLocation)) (LocalVariables|GetClosetDist))
      (LocalVariables|SetClosestActor _array_element)
      (LocalVariables|SetClosetDist (Math|Vector|Distance(Vector) (Transformation|GetActorLocation _array_element) (LocalVariables|GetPlayerLocation)))))
  (return (LocalVariables|GetClosestActor)))