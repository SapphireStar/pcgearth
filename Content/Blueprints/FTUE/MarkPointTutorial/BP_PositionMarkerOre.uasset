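; FTUE mark-point tutorial marker that positions itself on the ore nearest the player.
; GetTarget runs a large sphere overlap around the player pawn for MineSphereOre actors, picks the closest via GetClosestActor and moves the marker to its location.
; The event graph and construction script add no logic, so nothing in this Blueprint calls GetTarget.
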(event EventBeginPlay
  (|CallParentFunction) ; This node is disabled and will not be called.\nDrag off pins to build functionality.
)

(event Collision|EventActorBeginOverlap
  (params (OtherActor :type Actor%20Object%20Reference))
  (|CallParentFunction OtherActor) ; This node is disabled and will not be called.\nDrag off pins to build functionality.
)

(event EventTick
  (params (DeltaSeconds :type Float%20%28single-precision%29))
  (|CallParentFunction DeltaSeconds) ; This node is disabled and will not be called.\nDrag off pins to build functionality.
)

(fn ConstructionScript
  (|CallParentFunction))

(fn GetTarget
  (bind _outactors (Collision|SphereOverlapActors (Transformation|GetActorLocation (Game|Player|GetPlayerPawn 0)) 3e+04 (Utilities|Array|MakeArray "ObjectTypeQuery1" "ObjectTypeQuery2") "/Script/PCG.MineSphereOre"))
  (bind _output (CallFunction|GetClosestActor _outactors))
  (Transformation|SetActorLocation (Transformation|GetActorLocation _output) false false))