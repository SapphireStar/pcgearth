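; BP_PositionMarkerMainBuilding is an FTUE tutorial position marker for the main building.
; On BeginPlay it runs the parent logic, then sets its trigger distance.
; GetTarget finds a BP_MainBuilding actor by class and moves the marker to that actor's location.
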(event EventBeginPlay
  (|CallParentFunction)
  (Variables|Default|SetTriggerDistance 3.5e+03))

(event Collision|EventActorBeginOverlap
  (params (OtherActor :type Actor%20Object%20Reference))
  (|CallParentFunction OtherActor) ; This node is disabled and will not be called.\nDrag off pins to build functionality.
)

(event EventTick
  (params (DeltaSeconds :type Float%20%28single-precision%29))
  (|CallParentFunction DeltaSeconds) ; This node is disabled and will not be called.\nDrag off pins to build functionality.
)

(fn ConstructionScript
  (|CallParentFunction))

(fn GetTarget
  (bind _returnvalue (Actor|GetActorOfClass "/Game/Blueprints/Interactable/BP_MainBuilding.BP_MainBuilding_C"))
  (Transformation|SetActorLocation (Transformation|GetActorLocation _returnvalue) false false))