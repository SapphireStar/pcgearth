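; BP_MainBuilding is the player's central temple, marked by a Citadel mark point widget above it.
; Entering its box shows the submit popup and refills the player's fuel to max.
; Temple stage changes feed BuildLayer, which uses Wave Function Collapse to generate a layer from that stage's cache, offset in height by index.
; A time-zero game over event from PlayerData reinitializes the WFC core.
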(event OnComponentBeginOverlap(Box)
  (params (OverlappedComponent :type Primitive%20Component%20Object%20Reference) (OtherActor :type Actor%20Object%20Reference) (OtherComp :type Primitive%20Component%20Object%20Reference) (OtherBodyIndex :type Integer) (bFromSweep :type Boolean) (SweepResult :type Hit%20Result%20Structure%20%28by%20ref%29))
  (bind _gamemode (CallFunction|GetPCGGameMode))
  (bind _playerdata (Variables|/Script/PCG.PCGGameMode|GetPlayerData _gamemode))
  (if (== OtherActor (Game|Player|GetPlayerPawn 0))
    (Class|PCGGameMode|ShowPopup _gamemode "SubmitPopup")
    (Class|PlayerDataComponent|ChangePlayerAbilityPropertyValue _playerdata "EPAPT_CurrentFuel" (Class|PlayerDataComponent|GetPlayerAbilityPropertyValue _playerdata "EPAPT_FuelMax"))))

(event OnComponentEndOverlap(Box)
  (params (OverlappedComponent :type Primitive%20Component%20Object%20Reference) (OtherActor :type Actor%20Object%20Reference) (OtherComp :type Primitive%20Component%20Object%20Reference) (OtherBodyIndex :type Integer)))

(event Custom|CustomEvent
  (params (DataClassType :type Object%20Class%20Reference) (eGameOverType :type EGameOverType%20Enum :default "EGOT_Win"))
  (bind _wfcgenerator (Variables|Default|GetWFCGenerator))
  (Class|WFCGeneratorComponent|InitializeWFCCore _wfcgenerator (Variables|/Script/PCG.WFCGeneratorComponent|GetConfiguration _wfcgenerator)))

(event EventBeginPlay
  (bind _returnvalue (Game|ConstructObjectfromClass "/Game/Blueprints/UI/WBP_MarkPoint.WBP_MarkPoint_C"))
  (UserInterface|Viewport|AddtoViewport _returnvalue 0)
  (Default|InitializeMarkPoint _returnvalue "/Game/Textures/ScifiUI/Sci-fi_Icon_Pack___Free_iconset__Community___4_/citadel.citadel" (+ (Transformation|GetActorLocation) (* (Transformation|GetActorUpVector) 1e+03)))
  (EventDispatchers|BindEventtoOnCurrentTempleStageChanged (Variables|/Script/PCG.PCGGameMode|GetPlayerData (CallFunction|GetPCGGameMode)) (EventDispatchers|CreateEvent :!event OnTempleStageChanged))
  (EventDispatchers|BindEventtoOnTimeZeroGameOver (Variables|/Script/PCG.PCGGameMode|GetPlayerData (CallFunction|GetPCGGameMode)) (delegate Custom|CustomEvent)))

(event EventTick
  (params (DeltaSeconds :type Float%20%28single-precision%29)))

(fn ConstructionScript)

(fn GetPCGGameMode
  (bind _gamemode (Variables|Default|GetGameMode)
    (:then
      (return _gamemode))
    (:else
      (bind _asbp_pcggame_mode (Utilities|Casting|CastToBP_PCGGameMode (Game|GetGameMode)))
      (bind _output_get (Variables|Default|SetGameMode _asbp_pcggame_mode))
      (return _output_get))))

(fn BuildLayer
  (params (A :type Integer))
  (bind _wfcgenerator (Variables|Default|GetWFCGenerator))
  (bind _caches (Variables|Default|GetCaches))
  (bind _output (Utilities|Array|Get(acopy) _caches A))
  (bind _maxgridsize (Variables|/Script/PCG.WFCPreProcessCache|GetMaxGridSize _output))
  (Class|WFCGeneratorComponent|SetPreProcessCache (Variables|Default|GetWFCGenerator) _output)
  (Class|WFCGeneratorComponent|StartGenerationwithCustomGridSizeat _wfcgenerator (* (Math|Vector|VectorUp) (* A 500)) "0, 0, 0" (Utilities|Struct|MakeIntVector _maxgridsize _maxgridsize (.z (.gridsize (Variables|/Script/PCG.WFCGeneratorComponent|GetConfiguration _wfcgenerator))))))

(fn OnTempleStageChanged
  (params (OldValue :type Integer) (NewValue :type Integer))
  (CallFunction|BuildLayer OldValue))